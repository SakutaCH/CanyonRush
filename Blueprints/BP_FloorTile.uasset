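; BP_FloorTile is a floor tile that randomly decorates itself with either coins or one of three blocker variants, in left, center or right positions.
; Its Construction Script caches the three spawn point relative transforms, then rolls a random integer to choose the spawn function.
; Each function adds one Child Actor Component at a randomly picked point, so every tile gets a single item.
; The event graph holds no active logic.
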(fn `SetSapwnPoints`
  (set `self.SpawnPoints` (`|MakeArray` (`SceneComponent.GetRelativeTransform` (`self.SpawnPointL`)) (`SceneComponent.GetRelativeTransform` (`self.SpawnPointC`)) (`SceneComponent.GetRelativeTransform` (`self.SpawnPointR`)))))

(fn `SpawnBlocker`
  (bind _spawnpoints (`self.SpawnPoints`))
  (`AddComponent|NODE_AddChildActorComponent-0` :`RelativeTransform` (`|GetArrayItem` _spawnpoints (`KismetMathLibrary.RandomIntegerInRange` 0 (`KismetArrayLibrary.Array_LastIndex` _spawnpoints)))))

(fn `SpawnBlocker1`
  (bind _spawnpoints (`self.SpawnPoints`))
  (`AddComponent|NODE_AddChildActorComponent-4` :`RelativeTransform` (`|GetArrayItem` _spawnpoints (`KismetMathLibrary.RandomIntegerInRange` 0 (`KismetArrayLibrary.Array_LastIndex` _spawnpoints)))))

(fn `SpawnBlocker2`
  (bind _spawnpoints (`self.SpawnPoints`))
  (`AddComponent|NODE_AddChildActorComponent-5` :`RelativeTransform` (`|GetArrayItem` _spawnpoints (`KismetMathLibrary.RandomIntegerInRange` 0 (`KismetArrayLibrary.Array_LastIndex` _spawnpoints)))))

(fn `SpawnCoins`
  (bind _spawnpoints (`self.SpawnPoints`))
  (`AddComponent|NODE_AddChildActorComponent-3` :`RelativeTransform` (`|GetArrayItem` _spawnpoints (`KismetMathLibrary.RandomIntegerInRange` 0 (`KismetArrayLibrary.Array_LastIndex` _spawnpoints)))))

(fn `UserConstructionScript`
  (`self.SetSapwnPoints`)
  (switch `int` (`KismetMathLibrary.RandomIntegerInRange` 0 3)
    (:`Default`
      ;[1 1 1] Препятствия
      (`self.SpawnBlocker` :!label _label))
    (:`0`
      ;[1 1 1] Монеты
      (`self.SpawnCoins`))
    (:`1`
      (goto _label))
    (:`2`
      (`self.SpawnBlocker1`))
    (:`3`
      (`self.SpawnBlocker2`))))